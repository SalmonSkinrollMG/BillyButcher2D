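; BP_EnemyBase is an enemy base Blueprint that exposes combat targeting and attack animation events.
; SetCombatTarget writes the target to the Blackboard of the enemy's controller, using a key name variable.
; Attack plays a configurable sequence as an animation override on the PaperZD anim instance, if that sequence is valid.
; BeginPlay, overlap, Tick and the construction script add no logic of their own.
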(event EventBeginPlay
  (|CallParentFunction) ; This node is disabled and will not be called.\nDrag off pins to build functionality.
)

(event Collision|EventActorBeginOverlap
  (params (OtherActor :type Actor%20Object%20Reference))
  (|CallParentFunction OtherActor) ; This node is disabled and will not be called.\nDrag off pins to build functionality.
)

(event EventTick
  (params (DeltaSeconds :type Float%20%28single-precision%29))
  (|CallParentFunction DeltaSeconds) ; This node is disabled and will not be called.\nDrag off pins to build functionality.
)

(event EventSetCombatTarget
  (params (Target :type Actor%20Object%20Reference))
  (AI|Components|Blackboard|SetValueasObject (AI|GetBlackboard (Pawn|GetController)) (Variables|Default|GetKey%20Name) Target))

(event EventAttack
  (bind _attackanimsequence (Variables|Default|GetAttackAnimSequence)
    (:then
      (Class|PaperZDAnimInstance|PlayAnimationOverride (Variables|/Script/PaperZD.PaperZDAnimationComponent|GetAnimInstance (Variables|Default|GetPaperZDAnimation)) _attackanimsequence "DefaultSlot" 1.0 0.0))
    (:else)))

(fn ConstructionScript
  (|CallParentFunction))