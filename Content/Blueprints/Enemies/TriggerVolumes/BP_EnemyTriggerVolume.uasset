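; BP_EnemyTriggerVolume is a box trigger volume that tells a group of enemies when to target a player.
; When an actor implementing BPI_Player enters the box, each entry in OverlappingEnemies receives that actor through SetCombatTargetMessage.
; When such an actor leaves, the same message is sent without a target to clear it.
; The graph only reads the OverlappingEnemies list and never fills it.
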(event OnComponentBeginOverlap(Box)
  (params (OverlappedComponent :type Primitive%20Component%20Object%20Reference) (OtherActor :type Actor%20Object%20Reference) (OtherComp :type Primitive%20Component%20Object%20Reference) (OtherBodyIndex :type Integer) (bFromSweep :type Boolean) (SweepResult :type Hit%20Result%20Structure%20%28by%20ref%29))
  (if (and (Utilities|DoesObjectImplementInterface OtherActor "/Game/Blueprints/Interface/BPI_Player.BPI_Player_C") (> (Utilities|Array|Length (Variables|Default|GetOverlappingEnemies)) 0))
    (for _array_element (Variables|Default|GetOverlappingEnemies)
      (Class|BPIEnemy|SetCombatTarget(Message) _array_element OtherActor))))

(event OnComponentEndOverlap(Box)
  (params (OverlappedComponent :type Primitive%20Component%20Object%20Reference) (OtherActor :type Actor%20Object%20Reference) (OtherComp :type Primitive%20Component%20Object%20Reference) (OtherBodyIndex :type Integer))
  (if (and (Utilities|DoesObjectImplementInterface OtherActor "/Game/Blueprints/Interface/BPI_Player.BPI_Player_C") (> (Utilities|Array|Length (Variables|Default|GetOverlappingEnemies)) 0))
    (for _array_element (Variables|Default|GetOverlappingEnemies)
      (Class|BPIEnemy|SetCombatTarget(Message) _array_element))))

(fn ConstructionScript)