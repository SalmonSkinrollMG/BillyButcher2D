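; Behavior tree task that makes an AI-controlled enemy attack its combat target.
; It first snaps the pawn's yaw toward the CombatTarget actor read from the blackboard.
; It then calls AttackMessage on the pawn and immediately finishes successfully, without waiting for the attack to complete.
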(event EventReceiveExecuteAI
  (params (OwnerController :type AI%20Controller%20Object%20Reference) (ControlledPawn :type Pawn%20Object%20Reference))
  (CallFunction|RotateEnemyBasedonCharacter ControlledPawn)
  (Class|BPIEnemy|Attack(Message) ControlledPawn)
  (AI|BehaviorTree|FinishExecute true))

(fn RotateEnemyBasedonCharacter
  (params (ControlledPawn :type Actor%20Object%20Reference))
  (Transformation|SetActorRotation ControlledPawn (Math|Rotator|MakeRotator 0.0 0.0 (.yaw (Math|Rotator|MakeRotfromX (Math|Vector|Normalize (- (Transformation|GetActorLocation (AI|BehaviorTree|GetBlackboardValueasActor (Variables|Default|GetCombatTarget))) (Transformation|GetActorLocation ControlledPawn)) 0.1))))))