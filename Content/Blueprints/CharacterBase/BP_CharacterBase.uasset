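; Base character Blueprint for a PaperZD-animated character that reacts to being hit and can show damage numbers.
; On BeginPlay it caches its PlayerController, stopping if there is none, then creates a damage widget in the viewport when HasHitUi is set.
; HitReact plays an override animation and effect, subtracts the attacker's CurrentDamage from health, and animates and repositions the damage number.
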(event EventBeginPlay
  (bind _asplayer_controller (Utilities|Casting|CastToPlayerController (Pawn|GetController)))
  (Variables|Default|SetAs%20Player%20Controller _asplayer_controller)
  (CallFunction|CreateHitUI))

(event Collision|EventActorBeginOverlap
  (params (OtherActor :type Actor%20Object%20Reference)))

(event EventTick
  (params (DeltaSeconds :type Float%20%28single-precision%29)))

(event EventHitReact
  (params (AttackingActor :type BP%20Character%20Base%20Object%20Reference))
  (Class|PaperZDAnimInstance|PlayAnimationOverride (Variables|/Script/PaperZD.PaperZDAnimationComponent|GetAnimInstance (Variables|Default|GetPaperZDAnimation)) (Variables|HitReact|GetHitReactAnimSequence) "DefaultSlot" 1.0 0.0)
  (Niagara|SpawnSystematLocation (Variables|HitReact|GetHitReactFX) (Transformation|GetActorLocation))
  (CallFunction|ReduceHealth AttackingActor)
  (CallFunction|UpdateDamageUi (Variables|BP_CharacterBase_C|GetCurrentDamage AttackingActor)))

(fn ConstructionScript)

(fn ReduceHealth
  (params (AttackingActor :type BP%20Character%20Base%20Object%20Reference))
  (Variables|Default|SetCharacterHealth (- (Variables|Default|GetCharacterHealth) (Variables|BP_CharacterBase_C|GetCurrentDamage AttackingActor))))

(fn UpdateDamageUi
  (params (AttackerDamage :type Float%20%28double-precision%29))
  (bind _damageui (Variables|Default|GetDamageUI))
  (if (Variables|Default|GetHasHitUi)
    (Default|ShowText _damageui)
    (UserInterface|Animation|PlayAnimation _damageui (Variables|/Game/Blueprints/UI/DamageUi.DamageUi_C|GetDamageAnimation _damageui) 0.0 1 "Forward" 1.0 true)
    (Default|UpdateDamageNumber (Variables|Default|GetDamageUI) AttackerDamage)
    (Default|UpdatewidgetPosiiton (Variables|Default|GetDamageUI) self (Variables|Default|GetAs%20Player%20Controller))))

(fn CreateHitUI
  (if (Variables|Default|GetHasHitUi)
    (bind _returnvalue (UserInterface|CreateWidget "/Game/Blueprints/UI/DamageUi.DamageUi_C"))
    (bind _output_get (Variables|Default|SetDamageUI _returnvalue))
    (Default|UpdatewidgetPosiiton (Variables|Default|GetDamageUI) self (Variables|Default|GetAs%20Player%20Controller))
    (UserInterface|Viewport|AddtoViewport _output_get 10)))